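; BP_LevelLoading switches streaming sublevels, tracking a single active one by name in LevelLoaded.
; BeginPlay force-loads the level already named in LevelLoaded.
; LoadLevel skips repeat requests unless forced, clears the loaded and visible flags on the previous level, then sets them on the new one.
; An invalid name prints an on-screen error, except "None", which leaves no tracked level loaded.
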(event EventBeginPlay
  (CallFunction|LoadLevel (Variables|Default|GetLevel%20Loaded) true))

(fn ConstructionScript)

(fn LoadLevel
  (params (Level :type String) (Force :type Boolean))
  (if (or Force (Utilities|Enum|NotEqual(Enum) Level (Variables|Default|GetLevel%20Loaded)))
    (Utilities|FlowControl|Sequence
      (:then_0
        (Utilities|IsValid (Class|GameplayStatics|GetStreamingLevel (Utilities|String|StringToName (Variables|Default|GetLevel%20Loaded)))
          (:Is%20Valid
            (Variables|/Script/Engine.LevelStreaming|SetbShouldBeLoaded (Class|GameplayStatics|GetStreamingLevel (Utilities|String|StringToName (Variables|Default|GetLevel%20Loaded))) false)
            (Variables|/Script/Engine.LevelStreaming|SetbShouldBeVisible (Class|GameplayStatics|GetStreamingLevel (Utilities|String|StringToName (Variables|Default|GetLevel%20Loaded))) false))))
      (:then_1
        (bind _output_get (Variables|Default|SetLevel%20Loaded Level))
        (Utilities|IsValid (Class|GameplayStatics|GetStreamingLevel (Utilities|String|StringToName _output_get))
          (:Is%20Valid
            (Variables|/Script/Engine.LevelStreaming|SetbShouldBeLoaded (Class|GameplayStatics|GetStreamingLevel (Utilities|String|StringToName _output_get)) true)
            (Variables|/Script/Engine.LevelStreaming|SetbShouldBeVisible (Class|GameplayStatics|GetStreamingLevel (Utilities|String|StringToName _output_get)) true))
          (:Is%20Not%20Valid
            (if (Utilities|Enum|NotEqual(Enum) (Variables|Default|GetLevel%20Loaded) "None")
              (Development|PrintString (Utilities|String|Append "Error - LoadLevel - Invalid Level Name" (Variables|Default|GetLevel%20Loaded)) true true "(R=1.000000,G=0.015156,B=0.000000,A=1.000000)"))))))))