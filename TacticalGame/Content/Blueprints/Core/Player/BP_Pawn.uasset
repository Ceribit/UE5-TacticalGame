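; Player camera pawn that the player moves, rotates and zooms on a spring arm.
; Enhanced Input actions only update desired location, rotation and clamped zoom: movement follows the actor's forward and right vectors, and rotation turns in 45-degree steps.
; Tick smoothly interpolates the actor transform and spring arm length toward those targets, without sweeping for collision.
; The click action only prints its value.
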(event Input|EnhancedActionEvents|EnhancedInputActionIA_Zoom
  (params (ActionValue :type Float%20%28double-precision%29) (ElapsedSeconds :type Float%20%28double-precision%29) (TriggeredSeconds :type Float%20%28double-precision%29) (InputAction :type Input%20Action%20Object%20Reference :default "/Game/Blueprints/Core/Player/Input/IA_Zoom.IA_Zoom"))
  (:Triggered
    (Variables|Default|SetZoom_Desired (Math|Float|Clamp(Float) (+ (* ActionValue 1e+02) (Variables|Default|GetZoom_Desired)) 1e+02 5e+03))))

(event Input|EnhancedActionEvents|EnhancedInputActionIA_Click
  (params (ActionValue :type Boolean) (ElapsedSeconds :type Float%20%28double-precision%29) (TriggeredSeconds :type Float%20%28double-precision%29) (InputAction :type Input%20Action%20Object%20Reference :default "/Game/Blueprints/Core/Player/Input/IA_Click.IA_Click"))
  (:Triggered
    (Development|PrintString (Utilities|String|ToString(Boolean) ActionValue))))

(event Input|EnhancedActionEvents|EnhancedInputActionIA_AxisRight
  (params (ActionValue :type Float%20%28double-precision%29) (ElapsedSeconds :type Float%20%28double-precision%29) (TriggeredSeconds :type Float%20%28double-precision%29) (InputAction :type Input%20Action%20Object%20Reference :default "/Game/Blueprints/Core/Player/Input/IA_AxisRight.IA_AxisRight"))
  (:Triggered
    (Variables|Default|SetLocation_Desired (+ (Variables|Default|GetLocation_Desired) (* (* 2e+01 ActionValue) (Transformation|GetActorRightVector))))))

(event Input|EnhancedActionEvents|EnhancedInputActionIA_AxisForward
  (params (ActionValue :type Float%20%28double-precision%29) (ElapsedSeconds :type Float%20%28double-precision%29) (TriggeredSeconds :type Float%20%28double-precision%29) (InputAction :type Input%20Action%20Object%20Reference :default "/Game/Blueprints/Core/Player/Input/IA_AxisForward.IA_AxisForward"))
  (:Triggered
    (Variables|Default|SetLocation_Desired (+ (Variables|Default|GetLocation_Desired) (* (* 2e+01 ActionValue) (Transformation|GetActorForwardVector))))))

(event Input|EnhancedActionEvents|EnhancedInputActionIA_RotationLeft
  (params (ActionValue :type Boolean) (ElapsedSeconds :type Float%20%28double-precision%29) (TriggeredSeconds :type Float%20%28double-precision%29) (InputAction :type Input%20Action%20Object%20Reference :default "/Game/Blueprints/Core/Player/Input/IA_RotationLeft.IA_RotationLeft"))
  (:Started
    (Variables|Default|SetRotation_Desired (Math|Rotator|CombineRotators (Variables|Default|GetRotation_Desired) "0.000000,45.000000,0.000000"))))

(event Input|EnhancedActionEvents|EnhancedInputActionIA_RotationRight
  (params (ActionValue :type Boolean) (ElapsedSeconds :type Float%20%28double-precision%29) (TriggeredSeconds :type Float%20%28double-precision%29) (InputAction :type Input%20Action%20Object%20Reference :default "/Game/Blueprints/Core/Player/Input/IA_RotationRight.IA_RotationRight"))
  (:Started
    (Variables|Default|SetRotation_Desired (Math|Rotator|CombineRotators (Variables|Default|GetRotation_Desired) "0.000000,-45.000000,0.000000"))))

(event EventBeginPlay
  (Input|AddMappingContext (PlayerController|LocalPlayerSubsystems|GetEnhancedInputLocalPlayerSubsystem (Game|GetPlayerController 0)) "/Game/Blueprints/Core/Player/Input/IMC_Default.IMC_Default" 0 "(bIgnoreAllPressedKeysUntilRelease=True,bForceImmediately=False)")
  (Variables|Default|SetLocation_Desired (Transformation|GetActorLocation))
  (Variables|Default|SetZoom_Desired (Variables|/Script/Engine.SpringArmComponent|GetTargetArmLength (Variables|Default|GetSpringArm)))
  (Variables|Default|SetRotation_Desired (Transformation|GetActorRotation)))

(event EventTick
  (params (DeltaSeconds :type Float%20%28single-precision%29))
  (Variables|/Script/Engine.SpringArmComponent|SetTargetArmLength (Variables|Default|GetSpringArm) (Math|Interpolation|FInterpTo (Variables|/Script/Engine.SpringArmComponent|GetTargetArmLength (Variables|Default|GetSpringArm)) (Variables|Default|GetZoom_Desired) DeltaSeconds 2.0))
  (Transformation|SetActorLocation (Math|Interpolation|VInterpTo (Transformation|GetActorLocation) (Variables|Default|GetLocation_Desired) DeltaSeconds 5.0) false false)
  (Transformation|SetActorRotation (Math|Interpolation|RInterpTo (Transformation|GetActorRotation) (Variables|Default|GetRotation_Desired) DeltaSeconds 2.0)))

(fn ConstructionScript)