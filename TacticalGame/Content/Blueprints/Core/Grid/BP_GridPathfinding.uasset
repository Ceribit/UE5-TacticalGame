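; BP_GridPathfinding supplies tile neighbor queries for pathfinding on a grid, with no path search implemented yet.
; GetNeighborIndexes switches on the grid's tile shape to square, hexagon or triangle offset rules, with optional diagonals for squares and triangles.
; Hexagons use doubled-row offsets, and triangles use coordinate parity to pick their sideways neighbors.
; GetValidTileNeighbors keeps neighbors of walkable type whose height difference stays within the tile's Z size.
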(event EventBeginPlay)

(event Collision|EventActorBeginOverlap
  (params (OtherActor :type Actor%20Object%20Reference)))

(event EventTick
  (params (DeltaSeconds :type Float%20%28single-precision%29)))

(fn ConstructionScript)

(fn GetValidTileNeighbors
  (params (Index :type Int%20Point%20Structure) (IncludeDiagonals :type Boolean))
  (LocalVariables|SetInputData (.Value (Utilities|Map|Find (Variables|/Game/Blueprints/Core/Grid/BP_Grid.BP_Grid_C|GetGridTiles (Variables|Default|GetGrid)) Index)))
  (bind _neighbors (CallFunction|GetNeighborIndexes Index IncludeDiagonals))
  (for _array_element _neighbors
    (LocalVariables|SetData (.Value (Utilities|Map|Find (Variables|/Game/Blueprints/Core/Grid/BP_Grid.BP_Grid_C|GetGridTiles (Variables|Default|GetGrid)) _array_element)))
    (if (CallFunction|IsTileTypeWalkable (.type (LocalVariables|GetData)))
      (if (<= (Math|Float|Absolute(Float) (- (.z (.location (.transform (LocalVariables|GetData)))) (.z (.location (.transform (LocalVariables|GetInputData)))))) (.z (Variables|/Game/Blueprints/Core/Grid/BP_Grid.BP_Grid_C|GetGridTileSize (Variables|Default|GetGrid))))
        (Utilities|Array|Add (LocalVariables|GetRet) (.index (LocalVariables|GetData))))))
  (return (LocalVariables|GetRet)))

(fn GetNeighborIndexesforSquare
  (params (Index :type Int%20Point%20Structure) (IncludeDiagonals :type Boolean))
  (bind _returnvalue (Class|KismetMathLibrary|IntPointLeft))
  (bind _returnvalue_2 (Class|KismetMathLibrary|IntPointRight))
  (bind _returnvalue_3 (Class|KismetMathLibrary|IntPointUp))
  (bind _returnvalue_4 (Class|KismetMathLibrary|IntPointDown))
  (bind _returnvalue_5 (+ Index _returnvalue_3))
  (bind _returnvalue_6 (+ Index _returnvalue_4))
  (bind _returnvalue_7 (+ Index _returnvalue_2))
  (bind _returnvalue_8 (+ Index _returnvalue))
  (bind _array (Utilities|Array|MakeArray _returnvalue_5 _returnvalue_6 _returnvalue_8 _returnvalue_7))
  (if IncludeDiagonals
    (LocalVariables|SetRet _array)
    (Utilities|Array|AppendArray (LocalVariables|GetRet) (Utilities|Array|MakeArray (+ Index (Utilities|Struct|MakeIntPoint 1 1)) (+ Index (Utilities|Struct|MakeIntPoint -1 1)) (+ Index (Utilities|Struct|MakeIntPoint -1 -1)) (+ Index (Utilities|Struct|MakeIntPoint 1 -1))))
    (return (LocalVariables|GetRet))
    (else
      (return _array))))

(fn GetNeighborIndexesforHexagon
  (params (Index :type Int%20Point%20Structure))
  (return (Utilities|Array|MakeArray (+ Index (Utilities|Struct|MakeIntPoint 1 1)) (+ Index (Utilities|Struct|MakeIntPoint 0 2)) (+ Index (Utilities|Struct|MakeIntPoint -1 1)) (+ Index (Utilities|Struct|MakeIntPoint -1 -1)) (+ Index (Utilities|Struct|MakeIntPoint 0 -2)) (+ Index (Utilities|Struct|MakeIntPoint 1 -1)))))

(fn GetNeighborIndexesforTriangles
  (params (Index :type Int%20Point%20Structure) (IncludeDiagonals :type Boolean))
  (LocalVariables|SetRet (Utilities|Array|MakeArray (+ Index (Utilities|Struct|MakeIntPoint 0 1)) (+ Index (Utilities|Struct|MakeIntPoint 0 -1))))
  (if (== (CallFunction|IsIntEven (.x Index)) (CallFunction|IsIntEven (.y Index)))
    (Utilities|Array|Add (LocalVariables|GetRet) (+ Index (Utilities|Struct|MakeIntPoint -1 0)))
    (else
      (Utilities|Array|Add (LocalVariables|GetRet) (+ Index (Utilities|Struct|MakeIntPoint 1 0)))))
  (if IncludeDiagonals
    (if (== (CallFunction|IsIntEven (.x Index)) (CallFunction|IsIntEven (.y Index)))
      (Utilities|Array|AppendArray (LocalVariables|GetRet) (Utilities|Array|MakeArray (+ Index (Utilities|Struct|MakeIntPoint 1 0)) (+ Index (Utilities|Struct|MakeIntPoint -1 2)) (+ Index (Utilities|Struct|MakeIntPoint -1 -2))))
      (else
        (Utilities|Array|AppendArray (LocalVariables|GetRet) (Utilities|Array|MakeArray (+ Index (Utilities|Struct|MakeIntPoint -1 0)) (+ Index (Utilities|Struct|MakeIntPoint 1 2)) (+ Index (Utilities|Struct|MakeIntPoint 1 -2))))))
    (return (LocalVariables|GetRet))
    (else
      (return (LocalVariables|GetRet)))))

(fn GetNeighborIndexes
  (params (Index :type Int%20Point%20Structure) (IncludeDiagonals :type Boolean))
  (switch Utilities|FlowControl|Switch|SwitchonE_GridShape (Variables|/Game/Blueprints/Core/Grid/BP_Grid.BP_Grid_C|GetGridTileShape (Variables|Default|GetGrid))
    (:NewEnumerator1
      (return (CallFunction|GetNeighborIndexesforSquare Index IncludeDiagonals)))
    (:NewEnumerator2
      (return (CallFunction|GetNeighborIndexesforHexagon Index)))
    (:NewEnumerator3
      (return (CallFunction|GetNeighborIndexesforTriangles Index IncludeDiagonals)))))