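; BP_GridModifier is an editor-placed marker for grid tiles, carrying a shape and a tile type (None, Normal or Obstacle).
; The construction script sets the mesh from the shape's data and tints its material by type for visual feedback.
; It sets the mesh to overlap GameTraceChannel1 and hides the actor in game.
; The event graph holds no active logic.
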(event EventBeginPlay)

(event Collision|EventActorBeginOverlap
  (params (OtherActor :type Actor%20Object%20Reference)))

(event EventTick
  (params (DeltaSeconds :type Float%20%28single-precision%29)))

(fn ConstructionScript
  (bind _staticmesh (Variables|Default|GetStaticMesh))
  (Components|StaticMesh|SetStaticMesh _staticmesh (.mesh (CallFunction|GetShapeData (Variables|Default|GetShape))))
  (Rendering|Material|SetVectorParameterValueonMaterials _staticmesh "Color" (Math|Conversions|ToVector(LinearColor) (Utilities|Select :Index (Variables|Default|GetType) :NewEnumerator0 "" :NewEnumerator1 "(R=0.947307,G=0.947307,B=0.947307,A=1.000000)" :NewEnumerator2 "(R=0.863157,G=0.048172,B=0.061246,A=1.000000)")))
  (Collision|SetCollisionResponsetoChannel (Variables|Default|GetStaticMesh) "ECC_GameTraceChannel1" "ECR_Overlap")
  (Rendering|SetActorHiddenInGame true))